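; Door actor that swings open when the ThirdPersonCharacter enters its button trigger, if the Interupteur flag is set.
; The overlap starts a fast looping timer that calls OpenDoor, stepping ScenePorte's yaw one degree per call and clearing itself at 90.
; The construction script uses the same flag to toggle the button's visibility and Cylinder collision.
; Closing is unfinished: end overlap only casts, and nothing calls CloseDoor.
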(event OnComponentBeginOverlap(Trigger_Btn)
  (params (OverlappedComponent :type Primitive%20Component%20Object%20Reference) (OtherActor :type Actor%20Object%20Reference) (OtherComp :type Primitive%20Component%20Object%20Reference) (OtherBodyIndex :type Integer) (bFromSweep :type Boolean) (SweepResult :type Hit%20Result%20Structure%20%28by%20ref%29))
  (if (Variables|Default|GetInterupteur)
    (Utilities|Casting|CastToThirdPersonCharacter OtherActor)
    (bind _returnvalue (Utilities|Time|SetTimerbyEvent (delegate Custom|OpenDoor) 0.01 true))
    (Variables|Default|SetTimerDoor _returnvalue)
    (Development|PrintString "Hello")))

(event OnComponentEndOverlap(Trigger_Btn)
  (params (OverlappedComponent :type Primitive%20Component%20Object%20Reference) (OtherActor :type Actor%20Object%20Reference) (OtherComp :type Primitive%20Component%20Object%20Reference) (OtherBodyIndex :type Integer))
  (if (Variables|Default|GetInterupteur)
    (Utilities|Casting|CastToThirdPersonCharacter OtherActor)))

(event Custom|OpenDoor
  (bind _scene_porte (Variables|Default|GetScene_porte))
  (bind _relativerotation (Variables|/Script/Engine.SceneComponent|GetRelativeRotation _scene_porte))
  (bind _yaw (Math|Rotator|BreakRotator _relativerotation))
  (if (>= _yaw 9e+01)
    (if (Utilities|Time|IsValidTimerHandle (Variables|Default|GetTimerDoor))
      (Utilities|Time|ClearandInvalidateTimerbyHandle (Variables|Default|GetTimerDoor)))
    (else
      (Transformation|SetRelativeRotation _scene_porte (Math|Rotator|MakeRotator 0.0 0.0 (+ _yaw 1.0)) false false))))

(event Custom|CloseDoor
  (bind _scene_porte (Variables|Default|GetScene_porte))
  (bind _relativerotation (Variables|/Script/Engine.SceneComponent|GetRelativeRotation _scene_porte))
  (bind _yaw (Math|Rotator|BreakRotator _relativerotation))
  (if (>= _yaw 9e+01)
    (Transformation|SetRelativeRotation _scene_porte (Math|Rotator|MakeRotator 0.0 0.0 (+ _yaw -1.0)) false false)))

(event EventBeginPlay)

(event Collision|EventActorBeginOverlap
  (params (OtherActor :type Actor%20Object%20Reference)))

(event EventTick
  (params (DeltaSeconds :type Float%20%28single-precision%29)))

(fn ConstructionScript
  (if (Variables|Default|GetInterupteur)
    (Rendering|SetVisibility (Variables|Default|GetScene_Btn) true true)
    (Collision|SetCollisionEnabled (Variables|Default|GetCylinder) "QueryAndPhysics")
    (else
      (Collision|SetCollisionEnabled (Variables|Default|GetCylinder) "NoCollision")
      (Rendering|SetVisibility (Variables|Default|GetScene_Btn) false true))))